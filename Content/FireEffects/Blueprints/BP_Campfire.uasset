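; Campfire effect actor with a mesh, smoke and an animated light, each of which can be switched off per instance.
; The construction script hides the smoke, mesh or light rotator, along with the rotator's children, according to the Include flags.
; Each Tick adds a small relative rotation to the light rotator from game-time sine waves at different frequencies per axis, keeping the light moving without a timeline.
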(event EventTick
  (params (DeltaSeconds :type Float%20%28single-precision%29))
  (bind _returnvalue (Utilities|Time|GetGameTimeinSeconds))
  ;[1 1 1] Rotate Light
  (Transformation|AddRelativeRotation (Variables|Default|GetLightRotator) (Math|Rotator|MakeRotator (Math|Trig|Sin(Radians) (* _returnvalue 7.0)) (Math|Trig|Sin(Radians) _returnvalue) (Math|Trig|Sin(Radians) (* _returnvalue 3.0))) false false))

(fn ConstructionScript
  ;[1 1 1] Initial Setup
  (if (Variables|Default|GetIncludeSmoke)
    _
    (else
      (Rendering|SetVisibility (Variables|Default|GetP_Smoke) false false)))
  (if (Variables|Default|GetIncludeMesh)
    _
    (else
      (Rendering|SetVisibility (Variables|Default|GetCampfire) false false)))
  (if (not (Variables|Default|GetIncludeLight))
    (Rendering|SetVisibility (Variables|Default|GetLightRotator) false true)))