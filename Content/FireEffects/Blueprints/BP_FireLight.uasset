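; BP_FireLight is a fire light actor that wobbles a point light.
; The construction script applies colour, intensity, radius and a local X offset to PointLight1, then randomizes the LightRotator orientation and a speed multiplier.
; Each tick adds sine-driven rotation to LightRotator at different frequencies per axis.
; The random multiplier varies the motion between instances without animating intensity.
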(event EventTick
  (params (DeltaSeconds :type Float%20%28single-precision%29))
  (bind _returnvalue (Utilities|Time|GetGameTimeinSeconds))
  (bind _speed (Variables|Default|GetSpeed))
  (bind _randomvalue (Variables|Default|GetRandomValue))
  (bind _returnvalue_2 (* _returnvalue _speed))
  (bind _returnvalue_3 (* _returnvalue_2 _randomvalue))
  ;[1 1 1] Rotate Light
  (Transformation|AddRelativeRotation (Variables|Default|GetLightRotator) (Math|Rotator|MakeRotator (Math|Trig|Sin(Radians) (* _returnvalue_3 7.0)) (Math|Trig|Sin(Radians) _returnvalue_3) (Math|Trig|Sin(Radians) (* _returnvalue_3 3.0))) false false))

(fn ConstructionScript
  (bind _pointlight1 (Variables|Default|GetPointLight1))
  ;[1 1 1] Setup Light
  (Rendering|Components|Light|SetLightColor _pointlight1 (Variables|Default|GetLightColour) true)
  (Rendering|Components|Light|SetIntensity _pointlight1 (Variables|Default|GetLightIntensity))
  (Rendering|Lighting|SetAttenuationRadius _pointlight1 (Variables|Default|GetLightRadius))
  (Transformation|AddLocalOffset _pointlight1 (Math|Vector|MakeVector (Variables|Default|GetOffset) 0.0 0.0) false false)
  (Transformation|SetWorldRotation (Variables|Default|GetLightRotator) (Math|Random|RandomRotator true) false false)
  (Variables|Default|SetRandomValue (Math|Random|RandomFloatinRange 0.9 1.1)))